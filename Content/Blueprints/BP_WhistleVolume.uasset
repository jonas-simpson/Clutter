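; BP_WhistleVolume is a whistle area actor that follows the Cursor actor and grows while whistling is active.
; Each Tick it snaps to the cursor, scales the Cylinder from start to max size over TimeToMaxSize with a separate Z limit, and feeds the bounds to Niagara's Radius.
; SetIsWhistling toggles visibility, overlap events and Niagara, resetting hold time when off.
; Whistling switches itself off once hold time passes MaxHoldTime.
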(event EventBeginPlay)

(event Collision|EventActorBeginOverlap
  (params (OtherActor :type Actor%20Object%20Reference)))

(event EventTick
  (params (DeltaSeconds :type Float%20%28single-precision%29))
  (bind _startscale (Variables|Default|GetStartScale))
  (CallFunction|FollowCursor)
  (if (Variables|Default|GetIsWhistling)
    (bind _output_get (Variables|Default|SetCurrentHoldTime (+ DeltaSeconds (Variables|Default|GetCurrentHoldTime))))
    (if (> _output_get (Variables|Default|GetTimeToMaxSize))
      (if (> (Variables|Default|GetCurrentHoldTime) (Variables|Default|GetMaxHoldTime))
        (CallFunction|SetIsWhistling false))
      (else
        (Transformation|SetWorldScale3D (Variables|Default|GetCylinder) (Math|Vector|MakeVector (Math|Float|Lerp _startscale (Variables|Default|GetMaxScale) (Math|Float|MapRangeClamped (Variables|Default|GetCurrentHoldTime) 0.0 (Variables|Default|GetTimeToMaxSize) 0.0 1.0)) (Math|Float|Lerp _startscale (Variables|Default|GetMaxScale) (Math|Float|MapRangeClamped (Variables|Default|GetCurrentHoldTime) 0.0 (Variables|Default|GetTimeToMaxSize) 0.0 1.0)) (Math|Float|Lerp _startscale (Variables|Default|GetMaxScaleZ) (Math|Float|MapRangeClamped (Variables|Default|GetCurrentHoldTime) 0.0 (Variables|Default|GetTimeToMaxSize) 0.0 1.0))))
        (Niagara|SetNiagaraVariable(Float) (Variables|Default|GetNiagara) "Radius" (.x (.BoxExtent (Collision|GetComponentBounds (Variables|Default|GetCylinder)))))))))

(fn ConstructionScript)

(fn SetIsWhistling
  (params (IsWhistling :type Boolean))
  (bind _output_get (Variables|Default|SetIsWhistling IsWhistling))
  (Rendering|SetVisibility (Variables|Default|GetCylinder) _output_get true)
  (Variables|/Script/Engine.PrimitiveComponent|SetbGenerateOverlapEvents (Variables|Default|GetCylinder) _output_get)
  (Components|Activation|SetActive (Variables|Default|GetNiagara) IsWhistling true)
  (if (not IsWhistling)
    (Variables|Default|SetCurrentHoldTime 0.0)))

(fn FollowCursor
  (Transformation|SetActorLocation (Transformation|GetActorLocation (Variables|Default|GetCursor)) false false))