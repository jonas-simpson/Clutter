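; BP_CursorLine draws a line from the Clutter character's AimStart to the Clutter cursor, arching it while aiming.
; Each tick, UpdateSpline spaces points evenly between them, lifting the midpoint to character height plus AimHeight with widened tangents when Aiming.
; Two spline meshes follow the start, middle and end points, feeding center and radius to their materials.
; SetAiming also toggles the material's ShouldMarch parameter, while SetLineThickness scales both meshes.
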(event EventTick
  (params (DeltaSeconds :type Float%20%28single-precision%29))
  (CallFunction|UpdateSpline))

(event EventBeginPlay)

(fn ConstructionScript
  (Utilities|FlowControl|Sequence
    (:then_0
      (Variables|Default|SetPlayerComp (Variables|/Game/Blueprints/BP_ClutterCharacter.BP_ClutterCharacter_C|GetAimStart (CallFunction|GetClutterCharacter)))
      (Variables|Default|SetCursorComp (Variables|/Game/Blueprints/BP_ClutterCursor.BP_ClutterCursor_C|GetDefaultSceneRoot (CallFunction|GetClutterCursor))))
    (:then_1
      (CallFunction|SetLineThickness (Variables|Default|GetLineThickness)))))

(fn UpdateSpline
  (bind _startpoint (CallFunction|GetSplineStartPoint))
  (bind _midpoint (CallFunction|GetSplineMidpoint))
  (bind _endpoint (CallFunction|GetSplineEndpoint))
  (bind _midpoint_2 (CallFunction|GetSplineMidpoint))
  (bind _midpoint_3 (CallFunction|GetSplineMidpoint))
  (bind _playercomp (Variables|Default|GetPlayerComp))
  (bind _cursorcomp (Variables|Default|GetCursorComp))
  (bind _spline (Variables|Default|GetSpline))
  (bind _spline_2 (Variables|Default|GetSpline))
  (bind _spline_3 (Variables|Default|GetSpline))
  (bind (_inputkey _position _arrivetangent) (Utilities|Struct|BreakSplinePoint _midpoint))
  (bind (_inputkey_2 _position_2 _arrivetangent_2) (Utilities|Struct|BreakSplinePoint _endpoint))
  (bind _position_3 (Utilities|Struct|BreakSplinePoint _midpoint_2))
  (bind (_inputkey_3 _position_4 _arrivetangent_3 _leavetangent) (Utilities|Struct|BreakSplinePoint _midpoint_3))
  (bind (_inputkey_4 _position_5 _arrivetangent_4) (Utilities|Struct|BreakSplinePoint _startpoint))
  (bind _returnvalue (Transformation|GetWorldLocation _playercomp))
  (bind _returnvalue_2 (Transformation|GetWorldLocation _cursorcomp))
  (bind _returnvalue_3 (Spline|GetNumberOfSplinePoints _spline))
  (bind (_x _y _z) (Math|Vector|BreakVector _leavetangent))
  (bind (_x_2 _y_2 _z_2) (Math|Vector|BreakVector _arrivetangent_3))
  (bind _returnvalue_4 (- _returnvalue_3 1))
  (for _index (range 0 _returnvalue_4)
    (if (and (== (.Position (CallFunction|GetSplineMidpoint)) _index) (Variables|Default|GetAiming))
      (bind _output_get (Variables|Default|SetHighestPoint (Math|Vector|MakeVector (.X (Math|Vector|BreakVector (+ _returnvalue (* (Math|Vector|Normalize (- _returnvalue_2 _returnvalue)) (* (Math|Conversions|ToFloat(Integer) _index) (/ (Math|Vector|Distance(Vector) _returnvalue _returnvalue_2) (Math|Conversions|ToFloat(Integer) _returnvalue_4))))))) (.Y (Math|Vector|BreakVector (+ _returnvalue (* (Math|Vector|Normalize (- _returnvalue_2 _returnvalue)) (* (Math|Conversions|ToFloat(Integer) _index) (/ (Math|Vector|Distance(Vector) _returnvalue _returnvalue_2) (Math|Conversions|ToFloat(Integer) _returnvalue_4))))))) (+ (.z (Transformation|GetActorLocation (CallFunction|GetClutterCharacter))) (Variables|Default|GetAimHeight)))))
      (Spline|SetLocationatSplinePoint _spline_3 _index _output_get "Local" true)
      (Spline|SetSplinePointType _spline_2 _index "Curve" true)
      (Spline|SetTangentsatSplinePoint _spline_2 _index (Math|Vector|MakeVector (* _x_2 2.0) (* _y_2 2.0) _z_2) (Math|Vector|MakeVector (* _x 2.0) (* _y 2.0) _z) "Local" true)
      (else
        (Spline|SetLocationatSplinePoint _spline_3 _index (+ _returnvalue (* (Math|Vector|Normalize (- _returnvalue_2 _returnvalue)) (* (Math|Conversions|ToFloat(Integer) _index) (/ (Math|Vector|Distance(Vector) _returnvalue _returnvalue_2) (Math|Conversions|ToFloat(Integer) _returnvalue_4))))) "Local" true))))
  (SplineMesh|SetStartandEnd (Variables|Default|GetSplineMesh_First) _position_5 _arrivetangent_4 _position _arrivetangent true :!class /Script/Engine.SplineMeshComponent)
  (SplineMesh|SetStartandEnd (Variables|Default|GetSplineMesh_Second) _position _arrivetangent _position_2 _arrivetangent_2 true :!class /Script/Engine.SplineMeshComponent)
  (Rendering|Material|SetVectorParameterValueonMaterials (Variables|Default|GetSplineMesh_First) "SplineCenter" (.Position (Utilities|Struct|BreakSplinePoint (.Midpoint (CallFunction|GetSplineMidpoint)))))
  (Rendering|Material|SetScalarParameterValueonMaterials (Variables|Default|GetSplineMesh_First) "Radius" (* (Math|Vector|Distance(Vector) (.Position (Utilities|Struct|BreakSplinePoint (CallFunction|GetSplineStartPoint))) _position_3) 0.9))
  (Rendering|Material|SetScalarParameterValueonMaterials (Variables|Default|GetSplineMesh_Second) "Radius" (* (Math|Vector|Distance(Vector) _position_3 (.Position (Utilities|Struct|BreakSplinePoint (.EndPoint (CallFunction|GetSplineEndpoint))))) 0.9)))

(fn SetAiming
  (params (Aiming :type Boolean))
  (bind _output_get (Variables|Default|SetAiming Aiming))
  (CallFunction|UpdateMarchingMaterial _output_get)
  (if (not _output_get)
    (Spline|SetSplinePointType (Variables|Default|GetSpline) (.Position (CallFunction|GetSplineMidpoint)) "Curve" true)))

(fn GetSplineMidpoint
  (bind _spline (Variables|Default|GetSpline))
  (bind _returnvalue (Spline|GetNumberOfSplinePoints _spline))
  (bind _returnvalue_2 (- _returnvalue 1))
  (bind _returnvalue_3 (/ _returnvalue_2 2))
  (return (Spline|GetSplinePointAt _spline _returnvalue_3 "Local") _returnvalue_3))

(fn GetSplineStartPoint
  (return (Spline|GetSplinePointAt (Variables|Default|GetSpline) 0 "Local")))

(fn GetSplineEndpoint
  (bind _spline (Variables|Default|GetSpline))
  (bind _returnvalue (Spline|GetNumberOfSplinePoints _spline))
  (bind _returnvalue_2 (- _returnvalue 1))
  (return (Spline|GetSplinePointAt _spline _returnvalue_2 "Local") _returnvalue_2))

(fn ApplyLineThickness
  (bind _splinemesh_second (Variables|Default|GetSplineMesh_Second))
  (bind _linethickness (Variables|Default|GetLineThickness))
  (bind _returnvalue (Math|Conversions|ToVector2D(Vector) _linethickness))
  (SplineMesh|SetStartScale _splinemesh_second _returnvalue true :!class /Script/Engine.SplineMeshComponent)
  (SplineMesh|SetEndScale _splinemesh_second _returnvalue true :!class /Script/Engine.SplineMeshComponent))

(fn SetLineThickness
  (params (LineThickness :type Float%20%28double-precision%29))
  (Variables|Default|SetLineThickness (Math|Float|Lerp 0.0 0.0625 LineThickness))
  (CallFunction|ApplyLineThickness))

(fn UpdateMarchingMaterial
  (params (ShouldMarch :type Boolean))
  (Rendering|Material|SetScalarParameterValueonMaterials (Variables|Default|GetSplineMesh_First) "ShouldMarch" (Math|Conversions|ToFloat(Boolean) ShouldMarch)))