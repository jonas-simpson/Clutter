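; BP_StandaloneSpline is a Blueprint that turns a referenced spline into its own copy with a randomly nudged end point.
; On BeginPlay, if ReferenceSpline is valid, it rebuilds its Spline from that spline's world-space points, then clears the reference.
; It then offsets the last point by a short random vector, reading the position in local space but writing it as world space.
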(event EventBeginPlay
  (bind _spline (Variables|Default|GetSpline))
  (bind _returnvalue (Spline|GetNumberOfSplinePoints _spline))
  (bind _returnvalue_2 (- _returnvalue 1))
  (Utilities|IsValid (Variables|Default|GetReferenceSpline)
    (:Is%20Valid
      (Spline|ClearSplinePoints (Variables|Default|GetSpline) true)
      (for _index (range 0 (- (Spline|GetNumberOfSplinePoints (Variables|Default|GetReferenceSpline)) 1))
        (Class|SplineComponent|AddPoint (Variables|Default|GetSpline) (Spline|GetSplinePointAt (Variables|Default|GetReferenceSpline) _index "World") true))
      (Variables|Default|SetReferenceSpline 0)
      (Spline|SetLocationatSplinePoint (Variables|Default|GetSpline) _returnvalue_2 (+ (.position (Spline|GetSplinePointAt (Variables|Default|GetSpline) _returnvalue_2 "Local")) (* (Math|Random|RandomUnitVector) (Math|Random|RandomFloatinRange 1e+01 5e+01))) "World" true))))

(fn ConstructionScript)