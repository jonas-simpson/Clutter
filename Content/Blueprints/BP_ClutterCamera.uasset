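; Orbit camera for the Clutter character that follows a move target every tick, with smoothed yaw and pitch.
; Yaw speed eases in and out, while pitch interpolates along a vector curve that sets horizontal and vertical offsets, re-aiming the camera at LookTarget.
; SetShouldSnap starts a lerp that swings yaw behind the character.
; Input arrives through setter and start/end functions, as its own Enhanced Input logic is disconnected; debug prints remain.
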(event Input|EnhancedActionEvents|EnhancedInputActionIA_CameraYaw
  (params (ActionValue :type Float%20%28double-precision%29) (ElapsedSeconds :type Float%20%28double-precision%29) (TriggeredSeconds :type Float%20%28double-precision%29) (InputAction :type Input%20Action%20Object%20Reference :default "/Game/Input/IA_CameraYaw.IA_CameraYaw")))

(event Input|EnhancedActionEvents|EnhancedInputActionIA_CameraPitch
  (params (ActionValue :type Float%20%28double-precision%29) (ElapsedSeconds :type Float%20%28double-precision%29) (TriggeredSeconds :type Float%20%28double-precision%29) (InputAction :type Input%20Action%20Object%20Reference :default "/Game/Input/IA_CameraPitch.IA_CameraPitch")))

(event EventBeginPlay
  (CallFunction|OnPitchInputStart 0.01)
  (CallFunction|AddPitchInput 0.01 0.0025)
  (CallFunction|OnPitchInputEnd))

(event Collision|EventActorBeginOverlap
  (params (OtherActor :type Actor%20Object%20Reference)))

(event EventTick
  (params (DeltaSeconds :type Float%20%28single-precision%29))
  (CallFunction|AddYawInput (Variables|Yaw|GetYawInput) DeltaSeconds)
  (CallFunction|AddPitchInput (Variables|Pitch|GetPitchInput) DeltaSeconds)
  (Transformation|SetActorLocation (Transformation|GetActorLocation (Variables|Default|GetMoveTarget)) false false)
  (if (Variables|Default|GetSnapping)
    (CallFunction|SnapBehindPlayer DeltaSeconds)))

(fn ConstructionScript
  (bind _pitchfar (Variables|Default|GetPitchFar))
  (bind _pitchmid (Variables|Default|GetPitchMid))
  (bind _pitchclose (Variables|Default|GetPitchClose))
  (bind _camera (Variables|Default|GetCamera))
  (Utilities|FlowControl|Sequence
    (:then_0
      (Transformation|SetRelativeRotation _camera (CallFunction|GetLookRottoRoot (Transformation|GetWorldLocation _camera)) false false))
    (:then_1
      (Transformation|SetRelativeRotation _pitchfar (CallFunction|GetLookRottoRoot (Transformation|GetWorldLocation _pitchfar)) false false))
    (:then_2
      (Transformation|SetRelativeRotation _pitchmid (CallFunction|GetLookRottoRoot (Transformation|GetWorldLocation _pitchmid)) false false))
    (:then_3
      (Transformation|SetRelativeRotation _pitchclose (CallFunction|GetLookRottoRoot (Transformation|GetWorldLocation _pitchclose)) false false))))

(fn GetLookRottoRoot
  (params (SourceVec :type Vector))
  (return (Math|Rotator|FindLookatRotation SourceVec (Transformation|GetWorldLocation (Variables|Default|GetLookTarget)))))

(fn AddYawInput
  (params (Val :type Float%20%28double-precision%29) (DeltaTime :type Float%20%28double-precision%29))
  ;[0 1 0] Debug input
  (Development|PrintString (Class|KismetStringLibrary|BuildStringDouble "Camera X: " "" Val) true true "(R=0.000000,G=0.660000,B=1.000000,A=1.000000)" 0.001)
  ;[0 0 0] Calculate this frame's yaw speed
  (bind _output_get (Variables|Yaw|SetCurrentYawSpeed (Math|Interpolation|FInterpTo (Variables|Yaw|GetCurrentYawSpeed) (* Val (Variables|Yaw|GetTargetYawSpeed)) DeltaTime (* (Variables|Yaw|GetYawAccelerate) (Variables|Yaw|GetYawAccelerateMultiplier)))))
  ;[0 0 0] Rotate
  (Transformation|AddRelativeRotation (Variables|Default|GetYaw) (Math|Rotator|MakeRotator 0.0 0.0 _output_get) false false))

(fn AddPitchInput
  (params (Val :type Float%20%28double-precision%29) (DeltaTime :type Float%20%28double-precision%29))
  (bind _pitchhorizontal (Variables|Default|GetPitchHorizontal))
  (bind _pitchvertical (Variables|Default|GetPitchVertical))
  (bind _camera (Variables|Default|GetCamera))
  (bind _relativelocation (Variables|/Script/Engine.SceneComponent|GetRelativeLocation _pitchhorizontal))
  (bind _relativelocation_2 (Variables|/Script/Engine.SceneComponent|GetRelativeLocation _pitchvertical))
  ;[0 1 0] Debug input
  (Development|PrintString (Class|KismetStringLibrary|BuildStringDouble "Camera Y: " "" Val) true true "(R=0.000000,G=0.660000,B=1.000000,A=1.000000)" 0.001)
  ;[0 0 0] Calculate this frame's pitch movement speed
  (bind _output_get (Variables|Pitch|SetCurrentPitchSpeed (Math|Interpolation|FInterpTo (Variables|Pitch|GetCurrentPitchSpeed) (Variables|Pitch|GetTargetPitchSpeed) DeltaTime (* (Variables|Pitch|GetPitchAccelerate) (Variables|Pitch|GetPitchAccelerateMultiplier)))))
  ;[0 0 0] Don't continue if no input
  (if (!= _output_get 0.0)
    ;[0 0 0] Calculate this frame's position on the pitch curve
    (bind _output_get_2 (Variables|Pitch|SetCurrentPitchAlpha (Math|Interpolation|FInterpTo (Variables|Pitch|GetCurrentPitchAlpha) (Variables|Pitch|GetTargetPitchAlpha) DeltaTime (Variables|Pitch|GetCurrentPitchSpeed))))
    (LocalVariables|SetCurrentPitchCurveVal (Math|Curves|GetVectorValue (Variables|Pitch|GetPitchCurve) _output_get_2))
    ;[0 0 0] Set pitch horizontal location
    (Transformation|SetRelativeLocation (Variables|Default|GetPitchHorizontal) (Math|Vector|MakeVector (.x (LocalVariables|GetCurrentPitchCurveVal)) (.y _relativelocation) (.z _relativelocation)) false false)
    ;[0 0 0] Set pitch vertical location
    (Transformation|SetRelativeLocation (Variables|Default|GetPitchVertical) (Math|Vector|MakeVector (.x _relativelocation_2) (.y _relativelocation_2) (.z (LocalVariables|GetCurrentPitchCurveVal))) false false)
    ;[0 0 0] Aim camera at target
    (Transformation|SetRelativeRotation _camera (Math|Rotator|MakeRotator 0.0 (.pitch (CallFunction|GetLookRottoRoot (Transformation|GetWorldLocation _camera))) 0.0) false false)))

(fn OnYawInputStart
  (Variables|Yaw|SetYawAccelerateMultiplier 1.0)
  (Variables|Yaw|SetTargetYawSpeed (Variables|Yaw|GetMaxYawSpeed)))

(fn OnYawInputEnd
  (Variables|Yaw|SetTargetYawSpeed 0.0)
  (Variables|Yaw|SetYawInput 0.0)
  (Variables|Yaw|SetYawAccelerateMultiplier 4.0))

(fn OnPitchInputStart
  (params (ActionValue :type Float%20%28double-precision%29))
  (Variables|Pitch|SetPitchAccelerateMultiplier 1.0)
  (Variables|Pitch|SetTargetPitchSpeed (Variables|Pitch|GetMaxPitchSpeed))
  (Variables|Pitch|SetTargetPitchAlpha ActionValue))

(fn OnPitchInputEnd
  (Variables|Pitch|SetTargetPitchSpeed 0.0)
  (Variables|Pitch|SetPitchInput 0.0)
  (Variables|Pitch|SetPitchAccelerateMultiplier 4.0))

(fn SetYawInput
  (params (YawInput :type Float%20%28double-precision%29))
  (Variables|Yaw|SetYawInput YawInput))

(fn SetPitchInput
  (params (PitchInput :type Float%20%28double-precision%29))
  (Variables|Pitch|SetPitchInput PitchInput))

(fn GetCameraForwardandRight
  (bind _camera (Variables|Default|GetCamera))
  (bind (_forwardvector _rightvector) (CallFunction|GetComponentForwardandRight _camera))
  (return _forwardvector _rightvector))

(fn PrepVecforInput
  (params (VectorIn :type Vector))
  (bind (_x _y) (Math|Vector|BreakVector VectorIn))
  (return (Math|Vector|Normalize (Math|Vector|MakeVector _x _y 0.0))))

(fn SnapBehindPlayer
  (params (DeltaTime :type Float%20%28double-precision%29))
  (bind _output_get (Variables|Default|SetCurrentSnapAlpha (Math|Interpolation|FInterpTo (Variables|Default|GetCurrentSnapAlpha) 1.0 DeltaTime (Variables|Default|GetSnapSpeed))))
  (Transformation|SetWorldRotation (Variables|Default|GetYaw) (Math|Rotator|Lerp(Rotator) (Variables|Default|GetSnapStartRot) (Variables|Default|GetSnapTargetRot) _output_get true) false false)
  (if (> (Variables|Default|GetCurrentSnapAlpha) 0.95)
    (Variables|Default|SetSnapping false)))

(fn SetShouldSnap
  (params (ShouldSnap :type Boolean))
  (bind _output_get (Variables|Default|SetShouldSnap ShouldSnap))
  (if _output_get
    (Variables|Default|SetSnapping true)
    (Variables|Default|SetCurrentSnapAlpha 0.0)
    (bind _output_get_2 (Variables|Default|SetSnapStartRot (Transformation|GetWorldRotation (Variables|Default|GetYaw))))
    (Variables|Default|SetSnapTargetRot (Math|Rotator|MakeRotator (.roll _output_get_2) (.pitch _output_get_2) (.yaw (Transformation|GetActorRotation (CallFunction|GetClutterCharacter)))))))

(fn SetSnapTarget
  (params (SnapTarget :type Vector))
  (Variables|Default|SetSnapTarget SnapTarget))