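; Blueprint function library of shared global getters for the Clutter game.
; It casts player controller 0 to BP_ClutterPlayerController, and the character, camera, cursor and cursor line getters all read through that controller.
; It also exposes hard-coded constants for gravity and Gigi's throw height.
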(fn GetClutterController
  (bind _asbp_clutter_player_controller (Utilities|Casting|CastToBP_ClutterPlayerController (Game|GetPlayerController 0)))
  (return _asbp_clutter_player_controller))

(fn GetGravity
  (return -9.8e+02))

(fn GetClutterCharacter
  (return (Default|GetCharacter (CallFunction|GetClutterController))))

(fn GetClutterCamera
  (return (Default|GetCamera (CallFunction|GetClutterController))))

(fn GetClutterCursor
  (return (Variables|/Game/Blueprints/BP_ClutterPlayerController.BP_ClutterPlayerController_C|GetPlayerCursor (CallFunction|GetClutterController))))

(fn GetGigiThrowHeight
  (return 3e+02))

(fn GetCursorLine
  (return (Variables|/Game/Blueprints/BP_ClutterPlayerController.BP_ClutterPlayerController_C|GetCursorLine (CallFunction|GetClutterController))))