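; BP_ClutterCharacter is a physics-driven character moved by forces on its capsule rather than a movement component.
; When grounded, OnWalkInput applies camera-relative acceleration, clamps horizontal speed and prints debug values.
; Each tick turns the capsule toward input while moving and derives Grounded from collected hit normals, clearing it only while the body moves.
; SetAiming shifts the AimStart height, and GetEnvNormal traces below the capsule for a surface normal.
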(event OnComponentHit(Capsule)
  (params (HitComponent :type Primitive%20Component%20Object%20Reference) (OtherActor :type Actor%20Object%20Reference) (OtherComp :type Primitive%20Component%20Object%20Reference) (NormalImpulse :type Vector :default "0, 0, 0") (Hit :type Hit%20Result%20Structure%20%28by%20ref%29))
  (Utilities|Array|AddUnique (Variables|Default|GetHitsThisFrame) Hit))

(event EventBeginPlay)

(event Collision|EventActorBeginOverlap
  (params (OtherActor :type Actor%20Object%20Reference)))

(event EventTick
  (params (DeltaSeconds :type Float%20%28single-precision%29))
  (bind _capsule (Variables|Default|GetCapsule))
  (bind _returnvalue (Transformation|GetWorldLocation _capsule))
  (CallFunction|ProcessHits)
  (if (> (CallFunction|GetCurrentMoveSpeed) 1.0)
    (Transformation|SetWorldRotation (Variables|Default|GetCapsule) (Math|Interpolation|RInterpTo (Transformation|GetWorldRotation _capsule) (Math|Rotator|FindLookatRotation _returnvalue (+ _returnvalue (Variables|Default|GetInputDirRelative))) DeltaSeconds (Variables|Default|GetRotSpeed)) false false)))

(fn ConstructionScript)

(fn OnWalkInput
  (params (ActionValue :type Vector%202D%20Structure) (CameraForward :type Vector) (CameraRight :type Vector))
  (bind _returnvalue (Math|Vector2D|Normalize2D ActionValue))
  (bind _returnvalue_2 (Math|Conversions|ToVector(Vector2D) _returnvalue))
  (if (Variables|Default|GetGrounded)
    (bind _output_get (Variables|Default|SetCurrentMoveInput ActionValue))
    (Development|PrintString (Class|KismetStringLibrary|BuildStringVector2d "Character Movement: " "" _output_get) true true "(R=1.000000,G=0.660000,B=0.000000,A=1.000000)" 0.001)
    (Development|PrintString (Class|KismetStringLibrary|BuildStringDouble "Move speed: " "" (CallFunction|GetCurrentMoveSpeed)) true true "(R=1.000000,G=0.660000,B=0.000000,A=1.000000)" 0.001)
    (if (> (CallFunction|GetCurrentMoveSpeed) (Variables|Default|GetMaxMoveSpeed))
      ;[0 0 0] Character is moving at max speed, do not input
      (CallFunction|SetCurrentMoveSpeed (Variables|Default|GetMaxMoveSpeed))
      (else
        (bind _output_get_2 (Variables|Default|SetInputDirRelative (+ (* CameraForward (.x _returnvalue_2)) (* CameraRight (.y _returnvalue_2)))))
        (Physics|AddForce (Variables|Default|GetCapsule) (* _output_get_2 (Variables|Default|GetMoveAccel)) "None" true)))))

(fn GetCurrentMoveSpeed
  (bind _capsule (Variables|Default|GetCapsule))
  (bind _returnvalue (Transformation|GetComponentVelocity _capsule))
  (return (Math|Vector2D|Vector2DLength (Math|Vector2D|MakeVector2D (.x _returnvalue) (.y _returnvalue)))))

(fn GetCurrentMoveDir
  (bind _capsule (Variables|Default|GetCapsule))
  (bind _returnvalue (Transformation|GetComponentVelocity _capsule))
  (bind _returnvalue_2 (Math|Vector2D|MakeVector2D (.x _returnvalue) (.y _returnvalue)))
  (bind _returnvalue_3 (Math|Vector2D|Normalize2D _returnvalue_2))
  (return (Math|Vector|MakeVector (.x _returnvalue_3) (.y _returnvalue_3) (.z _returnvalue))))

(fn GetEnvNormal
  (bind _capsule (Variables|Default|GetCapsule))
  (bind (_origin _boxextent) (Collision|GetComponentBounds _capsule))
  (bind _returnvalue (- _origin _boxextent))
  (bind _returnvalue_2 (- _origin (Math|Vector|MakeVector 0.0 0.0 (.z _returnvalue))))
  (bind (_outhit _returnvalue_3) (Collision|LineTraceByChannel _returnvalue_2 (- _returnvalue_2 (Math|Vector|MakeVector 0.0 0.0 1e+01)) "TraceTypeQuery1" false 0 "None"))
  (if _returnvalue_3
    (return (.normal _outhit))
    (else
      (Development|PrintString "No hit. character airborne"))))

(fn SetCurrentMoveSpeed
  (params (Speed :type Float%20%28double-precision%29))
  (bind _movedir (CallFunction|GetCurrentMoveDir))
  (bind _returnvalue (Math|Vector2D|MakeVector2D (.x _movedir) (.y _movedir)))
  (bind _returnvalue_2 (* _returnvalue Speed))
  (Physics|SetPhysicsLinearVelocity (Variables|Default|GetCapsule) (Math|Vector|MakeVector (.x _returnvalue_2) (.y _returnvalue_2) (.z _movedir)) false "None"))

(fn SetAiming
  (params (Aiming :type Boolean))
  (bind _returnvalue (Transformation|GetActorLocation))
  (bind _aimstart (Variables|Default|GetAimStart))
  (bind (_x _y _z) (Math|Vector|BreakVector _returnvalue))
  (bind _output_get (Variables|Default|SetAiming Aiming))
  (if _output_get
    (Transformation|SetWorldLocation _aimstart (Math|Vector|MakeVector _x _y (+ _z 75.0)) false false)
    (else
      (Transformation|SetWorldLocation _aimstart (Math|Vector|MakeVector _x _y (- _z 0.0)) false false))))

(fn ProcessHits
  (for _array_element (Variables|Default|GetHitsThisFrame)
    (if (> (Math|Vector|DotProduct (.Normal (Collision|BreakHitResult _array_element)) "0.000000,0.000000,1.000000") (Variables|Default|GetMaxWalkableSlope))
      (Variables|Default|SetGrounded true)
      (Utilities|Array|Clear (Variables|Default|GetHitsThisFrame))
      (return)))
  (if (CallFunction|GetIsPhysicsBodyMoving)
    (Variables|Default|SetGrounded false))
  (Utilities|Array|Clear (Variables|Default|GetHitsThisFrame))
  (return))

(fn GetIsPhysicsBodyMoving
  (return (> (Math|Vector|VectorLength (Transformation|GetComponentVelocity (Variables|Default|GetCapsule))) 0.01)))