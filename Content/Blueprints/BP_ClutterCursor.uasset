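; World-space cursor actor that follows the mouse, staying within a maximum horizontal range of the player character.
; Each tick a visibility trace along the mouse ray skips "IgnoreMouse"-tagged actors, cached at BeginPlay, whose BP_IgnoreMouse component is enabled.
; In-range points are height-capped by Gigi's throw height; others snap to the range edge, slightly below the character's origin.
; The location also feeds the MPC_GUI material parameter collection.
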(event EventBeginPlay
  (bind _outactors (Actor|GetAllActorswithTag "IgnoreMouse"))
  (Variables|Default|SetSpecialActors _outactors))

(event Collision|EventActorBeginOverlap
  (params (OtherActor :type Actor%20Object%20Reference)))

(event EventTick
  (params (DeltaSeconds :type Float%20%28single-precision%29))
  (bind _character (CallFunction|GetClutterCharacter))
  (bind _cluttercontroller (CallFunction|GetClutterController))
  (bind _character_2 (Variables|Default|GetCharacter))
  (bind (_worldlocation _worlddirection _returnvalue) (Game|Player|ConvertMouseLocationToWorldSpace _cluttercontroller))
  (bind _returnvalue_2 (Transformation|GetActorLocation _character))
  (bind _returnvalue_3 (Transformation|GetActorLocation _character_2))
  ;[0 0 0] Do we have a mouse position?
  (if _returnvalue
    ;[0 1 0] Comment
    (Development|PrintString "Mouse" true true "(R=0.000000,G=1.000000,B=0.000000,A=1.000000)" 0.01)
    ;[0 0 0] Get location of mouse point
    (bind _output_get (Variables|Default|SetMouseMaxPointLocation (+ _worldlocation (* _worlddirection (Variables|Default|GetCursorCheckLength)))))
    (bind _output_get_2 (Variables|Default|SetActorsToIgnore (CallFunction|GetActorstoIgnore)))
    (bind (_outhit _returnvalue_4) (Collision|LineTraceByChannel (+ _worldlocation (* _worlddirection (Variables|Default|GetCameraNearCheck))) _output_get "TraceTypeQuery1" false _output_get_2 "None"))
    (if _returnvalue_4
      (Variables|Default|SetMousePointLocation (.location _outhit))
      (else
        (Variables|Default|SetMousePointLocation (Variables|Default|GetMouseMaxPointLocation))))
    ;[0 0 0] Is it close enough to the player character?
    (if (<= (Math|Vector|Distance(Vector) (Math|Vector|MakeVector (.X (Math|Vector|BreakVector (Variables|Default|GetMousePointLocation))) (.Y (Math|Vector|BreakVector (Variables|Default|GetMousePointLocation))) 0.0) (Math|Vector|MakeVector (.x _returnvalue_2) (.y _returnvalue_2) 0.0)) (Variables|Default|GetMaxDistance))
      (Variables|Default|SetCursorLocation (Math|Vector|MakeVector (.X (Math|Vector|BreakVector (Variables|Default|GetMousePointLocation))) (.Y (Math|Vector|BreakVector (Variables|Default|GetMousePointLocation))) (Math|Float|Min(Float) (.Z (Math|Vector|BreakVector (Variables|Default|GetMousePointLocation))) (+ (.z (Transformation|GetActorLocation (Variables|Default|GetCharacter))) (CallFunction|GetGigiThrowHeight)))))
      (else
        ;[0 0 0] If not, simulate a new hit point on the ground
        (Variables|Default|SetCursorLocation (+ _returnvalue_3 (* (Math|Vector|Normalize (Math|Vector|MakeVector (.x (- (Variables|Default|GetMousePointLocation) _returnvalue_3)) (.y (- (Variables|Default|GetMousePointLocation) _returnvalue_3)) 0.0)) (Variables|Default|GetMaxDistance)) "0.000000,0.000000,-50.000000"))))
    ;[0 0 0] Set our cursor
    (Transformation|SetActorLocation (Variables|Default|GetCursorLocation) false false)
    (Rendering|Material|SetVectorParameterValue "/Game/Materials/MPC_GUI.MPC_GUI" "CursorLocation" (Math|Conversions|ToLinearColor(Vector) (Variables|Default|GetCursorLocation)) :!class /Script/Engine.KismetMaterialLibrary)
    (else
      (Development|PrintString "No Mouse" true true "(R=1.000000,G=0.000000,B=0.000000,A=1.000000)" 0.01))))

(fn ConstructionScript)

(fn GetActorstoIgnore
  (for _array_element (Variables|Default|GetSpecialActors)
    (bind _output_get (LocalVariables|SetCurrentComp (Actor|GetComponentbyClass _array_element "/Game/BP_IgnoreMouse.BP_IgnoreMouse_C")))
    (Utilities|IsValid _output_get
      (:Is%20Valid
        (if (Variables|/Game/BP_IgnoreMouse.BP_IgnoreMouse_C|GetEnabled (LocalVariables|GetCurrentComp))
          (Utilities|Array|Add (LocalVariables|GetActors) _array_element)))))
  (return (LocalVariables|GetActors)))