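; BP_ArtificialGravity is an actor component that applies scaled artificial gravity to its owning actor.
; On BeginPlay it caches the owner's root as a PrimitiveComponent, or prints an error and destroys itself if the cast fails.
; Each Tick it adds a vertical force of GetGravity times GravityScale as an acceleration change, so the effect is independent of mass.
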(event EventBeginPlay
  (bind _asprimitive_component (Utilities|Casting|CastToPrimitiveComponent (Variables|/Script/Engine.Actor|GetRootComponent (Components|GetOwner)))
    (:then
      (Variables|Default|SetOwner _asprimitive_component)
      (Development|PrintString "Primitive found!"))
    (:CastFailed
      (Development|PrintString "Cannot apply artivicial gravity to actor!! Make sure root component is Primitive" true true "(R=1.000000,G=0.000000,B=0.000000,A=1.000000)")
      (Components|DestroyComponent))))

(event EventTick
  (params (DeltaSeconds :type Float%20%28single-precision%29))
  (Physics|AddForce (Variables|Default|GetOwner) (Math|Vector|MakeVector 0.0 0.0 (* (CallFunction|GetGravity) (Variables|Default|GetGravityScale))) "None" true))