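; BP_GigiSquad manages the player character's squad of Gigis, tracking members and squad size and handling hold, throw and dismiss commands.
; The character's hold request picks the closest member, changes its state and snaps it to the GigiHold point.
; Throwing spawns a standalone spline from the cursor line as the Gigi's path, then removes it from the squad.
; Dismissing resets every member's state without emptying the list.
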(event Custom|ThrowRequest)

(event Custom|DismissRequest
  (for _array_element (Variables|Default|GetSquadMembers)
    (Variables|/Game/Blueprints/BP_Gigi.BP_Gigi_C|SetState _array_element "NewEnumerator0")))

(event Custom|HandleHoldRequest
  (bind _output_get (Variables|Default|SetGigiToThrow (CallFunction|GetClosestGigi)))
  (Default|SetState _output_get "NewEnumerator7")
  (Transformation|AttachComponentToComponent (Variables|Default|GetGigiToThrow) (Variables|/Game/Blueprints/BP_ClutterCharacter.BP_ClutterCharacter_C|GetGigiHold (Variables|Default|GetMyCharacter)) "None" "SnapToTarget" "SnapToTarget" "SnapToTarget" true))

(event Custom|ThrowGigi
  (Default|SetState (Variables|Default|GetGigiToThrow) "NewEnumerator6")
  (bind _returnvalue (Game|SpawnActorfromClass "/Game/Blueprints/BP_StandaloneSpline.BP_StandaloneSpline_C" (Math|Transform|MakeTransform "0, 0, 0" "0, 0, 0" "1.000000,1.000000,1.000000") "AlwaysSpawn" "MultiplyWithRoot" 0 (Variables|/Game/Blueprints/BP_CursorLine.BP_CursorLine_C|GetSpline (CallFunction|GetCursorLine)) 0))
  (Variables|/Game/Blueprints/BP_Gigi.BP_Gigi_C|SetMyThrowPath (Variables|Default|GetGigiToThrow) _returnvalue)
  (Default|Throw (Variables|Default|GetGigiToThrow))
  (CallFunction|RemoveGigifromSquad (Variables|Default|GetGigiToThrow))
  (Variables|Default|SetGigiToThrow 0))

(event EventBeginPlay
  (Utilities|IsValid (Variables|Default|GetMyCharacter)
    (:Is%20Valid
      (EventDispatchers|BindEventtoHoldRequest (Variables|Default|GetMyCharacter) (delegate Custom|HandleHoldRequest)))))

(fn ConstructionScript)

(fn GetClosestGigi
  (if (> (Variables|Default|GetSquadSize) 0)
    (LocalVariables|SetCharacterLocation (Transformation|GetActorLocation (Variables|Default|GetMyCharacter)))
    (for _array_element (Variables|Default|GetSquadMembers)
      (bind _output_get (LocalVariables|SetCurrentDist (Math|Vector|Distance(Vector) (Transformation|GetActorLocation _array_element) (LocalVariables|GetCharacterLocation))))
      (if (< _output_get (LocalVariables|GetMinDist))
        (LocalVariables|SetMinDist (LocalVariables|GetCurrentDist))
        (LocalVariables|SetClosestGigi _array_element)))
    (return (LocalVariables|GetClosestGigi))
    (else
      (return 0))))

(fn CheckIsEmpty
  (return (Utilities|Array|IsEmpty (Variables|Default|GetSquadMembers))))

(fn AddGigitoSquad
  (params (Gigi :type BP%20Gigi%20Object%20Reference))
  (Utilities|Array|Add (Variables|Default|GetSquadMembers) Gigi)
  (Math|Integer|IncrementInt (Variables|Default|GetSquadSize)))

(fn RemoveGigifromSquad
  (params (Gigi :type BP%20Gigi%20Object%20Reference))
  (bind _returnvalue (Utilities|Array|RemoveItem (Variables|Default|GetSquadMembers) Gigi))
  (if _returnvalue
    (Math|Integer|DecrementInt (Variables|Default|GetSquadSize))))