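; BPFL_ClutterMath is a small math helper library, named for clutter, that returns forward and right direction vectors.
; The actor function passes through the actor's forward and right vectors unchanged.
; The scene component function flattens both vectors onto the XY plane by zeroing Z, then renormalizes them, so only its results are guaranteed horizontal.
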(fn GetActorForwardandRightVectors
  (params (Actor :type Actor%20Object%20Reference))
  (return (Transformation|GetActorForwardVector Actor) (Transformation|GetActorRightVector Actor)))

(fn GetComponentForwardandRight
  (params (SceneComponent :type Scene%20Component%20Object%20Reference))
  (bind _returnvalue (Math|Vector|MakeVector 1.0 1.0 0.0))
  (return (Math|Vector|Normalize (* (Math|Vector|GetForwardVector SceneComponent) _returnvalue)) (Math|Vector|Normalize (* (Math|Vector|GetRightVector SceneComponent) _returnvalue))))