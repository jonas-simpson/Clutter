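; BP_Gigi is a squad follower that joins the Clutter character's squad when a whistle volume overlaps its capsule while idle.
; Joining sets the character as its move target and switches its state to In Squad, where Tick runs FollowMoveTarget.
; Following is physics-driven: the capsule yaws toward the target and gets horizontal acceleration until close, with horizontal speed capped at a maximum.
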(event OnComponentBeginOverlap(Capsule)
  (params (OverlappedComponent :type Primitive%20Component%20Object%20Reference) (OtherActor :type Actor%20Object%20Reference) (OtherComp :type Primitive%20Component%20Object%20Reference) (OtherBodyIndex :type Integer) (bFromSweep :type Boolean) (SweepResult :type Hit%20Result%20Structure%20%28by%20ref%29))
  (bind _character (CallFunction|GetClutterCharacter))
  (Utilities|Casting|CastToBP_WhistleVolume OtherActor)
  (switch Utilities|FlowControl|Switch|SwitchonE_GigiState (Variables|Default|GetState)
    (:NewEnumerator0
      (Default|AddGigitoSquad (Variables|/Game/Blueprints/BP_ClutterCharacter.BP_ClutterCharacter_C|GetMySquad _character) self)
      (Variables|Default|SetMoveTarget _character)
      (Variables|Default|SetState "NewEnumerator5"))))

(event EventTick
  (params (DeltaSeconds :type Float%20%28single-precision%29))
  (switch Utilities|FlowControl|Switch|SwitchonE_GigiState (Variables|Default|GetState)
    (:NewEnumerator5
      ;[0 0 0] Follow captain
      (CallFunction|FollowMoveTarget))))

(fn ConstructionScript)

(fn FollowMoveTarget
  ;[0 0 0] Get my and target locations
  (LocalVariables|SetMyLocation (Transformation|GetActorLocation))
  (LocalVariables|SetTargetLocation (Transformation|GetActorLocation (Variables|Default|GetMoveTarget)))
  ;[0 0 0] Rotate to face target
  (Transformation|SetWorldRotation (Variables|Default|GetCapsule) (Math|Rotator|MakeRotator 0.0 0.0 (.yaw (Math|Rotator|FindLookatRotation (LocalVariables|GetMyLocation) (LocalVariables|GetTargetLocation)))) false false)
  ;[0 0 0] Am I moving under the speed limit?
  (if (< (Math|Vector|VectorLength (Transformation|GetComponentVelocity (Variables|Default|GetCapsule))) (Variables|Default|GetMaxMoveSpeed))
    ;[0 0 0] Am I too close to the target?
    (if (not (< (Math|Vector|Distance(Vector) (LocalVariables|GetMyLocation) (LocalVariables|GetTargetLocation)) 2e+02))
      ;[0 0 0] Add force in direction of target
      (Physics|AddForce (Variables|Default|GetCapsule) (* (Math|Vector|MakeVector (.x (Math|Vector|GetUnitDirection(Vector) (LocalVariables|GetMyLocation) (LocalVariables|GetTargetLocation))) (.y (Math|Vector|GetUnitDirection(Vector) (LocalVariables|GetMyLocation) (LocalVariables|GetTargetLocation))) 0.0) (Variables|Default|GetMoveAccel)) "None" true))
    (else
      (CallFunction|SetComponentHorizontalVelocity (Variables|Default|GetCapsule) (Variables|Default|GetMaxMoveSpeed)))))