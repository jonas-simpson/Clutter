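; Player controller for the Clutter game that spawns and wires up the character, cursor, cursor line and whistle volume at the level's camera.
; Adds Enhanced Input contexts and routes camera yaw, pitch and snap, camera-relative walking, and whistling to those actors.
; Punch input drives aiming on the character and cursor line, with a delayed release that keeps the line arced between clicks.
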(event Custom|StopAimDelay
  ;[0 0 0] Delay after input ends to keep line in an arc between clicks
  (Utilities|FlowControl|Delay (Variables|Default|GetStop%20Aiming%20Delay))
  (if (not (Variables|Default|GetAiming))
    (if (Variables|Default|GetStopAimAttempt)
      (Variables|Default|SetStopAimAttempt false)
      (Default|SetAiming (Variables|Default|GetCursorLine) false)
      (Default|SetAiming (Variables|Default|GetPlayerCharacter) false)
      (else
        (Variables|Default|SetStopAimAttempt true)
        (CallFunction|StopAimDelay)))))

(event Input|EnhancedActionEvents|EnhancedInputActionIA_CameraYaw
  (params (ActionValue :type Float%20%28double-precision%29) (ElapsedSeconds :type Float%20%28double-precision%29) (TriggeredSeconds :type Float%20%28double-precision%29) (InputAction :type Input%20Action%20Object%20Reference :default "/Game/Input/IA_CameraYaw.IA_CameraYaw"))
  (bind _playercamera (Variables|Default|GetPlayerCamera))
  (:Triggered
    (Default|SetYawInput _playercamera ActionValue))
  (:Started
    (Default|OnYawInputStart _playercamera))
  (:Canceled
    (Default|OnYawInputEnd _playercamera :!label _label))
  (:Completed
    (goto _label)))

(event Input|EnhancedActionEvents|EnhancedInputActionIA_CameraPitch
  (params (ActionValue :type Float%20%28double-precision%29) (ElapsedSeconds :type Float%20%28double-precision%29) (TriggeredSeconds :type Float%20%28double-precision%29) (InputAction :type Input%20Action%20Object%20Reference :default "/Game/Input/IA_CameraPitch.IA_CameraPitch"))
  (bind _playercamera (Variables|Default|GetPlayerCamera))
  (:Triggered
    (Default|SetPitchInput _playercamera ActionValue))
  (:Started
    (Default|OnPitchInputStart _playercamera ActionValue))
  (:Canceled
    (Default|OnPitchInputEnd _playercamera :!label _label))
  (:Completed
    (goto _label)))

(event Input|EnhancedActionEvents|EnhancedInputActionIA_Walk
  (params (ActionValue :type Vector%202D%20Structure) (ElapsedSeconds :type Float%20%28double-precision%29) (TriggeredSeconds :type Float%20%28double-precision%29) (InputAction :type Input%20Action%20Object%20Reference :default "/Game/Input/IA_Walk.IA_Walk"))
  (bind _playercamera (Variables|Default|GetPlayerCamera))
  (bind (_cameraforward _cameraright) (Default|GetCameraForwardandRight _playercamera))
  (Default|OnWalkInput (Variables|Default|GetPlayerCharacter) ActionValue _cameraforward _cameraright))

(event Input|EnhancedActionEvents|EnhancedInputActionIA_CameraSnap
  (params (ActionValue :type Boolean) (ElapsedSeconds :type Float%20%28double-precision%29) (TriggeredSeconds :type Float%20%28double-precision%29) (InputAction :type Input%20Action%20Object%20Reference :default "/Game/Input/IA_CameraSnap.IA_CameraSnap"))
  (bind _playercamera (CallFunction|GetCamera))
  (:Triggered
    (Default|SetSnapTarget _playercamera (- "1.000000,1.000000,1.000000" (Transformation|GetActorForwardVector (CallFunction|GetCharacter)))))
  (:Started
    (Default|SetShouldSnap _playercamera true))
  (:Canceled
    (Default|SetShouldSnap _playercamera false :!label _label))
  (:Completed
    (goto _label)))

(event Input|EnhancedActionEvents|EnhancedInputActionIA_Punch
  (params (ActionValue :type Boolean) (ElapsedSeconds :type Float%20%28double-precision%29) (TriggeredSeconds :type Float%20%28double-precision%29) (InputAction :type Input%20Action%20Object%20Reference :default "/Game/Input/IA_Punch.IA_Punch"))
  (:Started
    (Variables|Default|SetAiming true)
    (Variables|Default|SetStopAimAttempt false)
    (Default|SetAiming (Variables|Default|GetCursorLine) true)
    (Default|SetAiming (Variables|Default|GetPlayerCharacter) true))
  (:Canceled
    (Variables|Default|SetAiming false :!label _label)
    (if (Variables|Default|GetStopAimAttempt)
      (Variables|Default|SetStopAimAttempt false)
      (Default|SetAiming (Variables|Default|GetCursorLine) false)
      (Default|SetAiming (Variables|Default|GetPlayerCharacter) false)
      (else
        (Variables|Default|SetStopAimAttempt true)
        (CallFunction|StopAimDelay))))
  (:Completed
    (goto _label)))

(event Input|EnhancedActionEvents|EnhancedInputActionIA_Whistling
  (params (ActionValue :type Boolean) (ElapsedSeconds :type Float%20%28double-precision%29) (TriggeredSeconds :type Float%20%28double-precision%29) (InputAction :type Input%20Action%20Object%20Reference :default "/Game/Input/IA_Whistling.IA_Whistling"))
  (:Started
    (Default|SetIsWhistling (Variables|Default|GetWhistleVolume) true))
  (:Canceled
    (Default|SetIsWhistling (Variables|Default|GetWhistleVolume) false :!label _label))
  (:Completed
    (goto _label)))

(event EventBeginPlay
  (bind _self self)
  (bind _returnvalue (PlayerController|LocalPlayerSubsystems|GetEnhancedInputLocalPlayerSubsystem _self))
  (Utilities|FlowControl|Sequence
    (:then_0
      (bind _returnvalue_2 (Actor|GetActorOfClass "/Game/Blueprints/BP_ClutterCamera.BP_ClutterCamera_C"))
      (bind _output_get (Variables|Default|SetPlayerCamera _returnvalue_2))
      (bind _returnvalue_3 (Game|SpawnActorfromClass "/Game/Blueprints/BP_ClutterCharacter.BP_ClutterCharacter_C" (Math|Transform|MakeTransform (+ (.location (Transformation|GetActorTransform _output_get)) "0.000000,0.000000,50.000000") (.rotation (Transformation|GetActorTransform _output_get)) "1.000000,1.000000,1.000000") "AlwaysSpawn" "MultiplyWithRoot" 0 0))
      (bind _output_get_2 (Variables|Default|SetPlayerCharacter _returnvalue_3))
      (bind _returnvalue_4 (Game|SpawnActorfromClass "/Game/Blueprints/BP_ClutterCursor.BP_ClutterCursor_C" (Math|Transform|MakeTransform (Transformation|GetActorLocation _output_get_2) "0, 0, 0" "1.000000,1.000000,1.000000") "Undefined" "MultiplyWithRoot" 0 (Variables|Default|GetPlayerCharacter) 0))
      (Variables|Default|SetPlayerCursor _returnvalue_4)
      (bind _returnvalue_5 (Game|SpawnActorfromClass "/Game/Blueprints/BP_CursorLine.BP_CursorLine_C" (Math|Transform|MakeTransform "0, 0, 0" "0, 0, 0" "1.000000,1.000000,1.000000") "Undefined" "MultiplyWithRoot" 0 0))
      (Variables|Default|SetCursorLine _returnvalue_5)
      (bind _returnvalue_6 (Game|SpawnActorfromClass "/Game/Blueprints/BP_WhistleVolume.BP_WhistleVolume_C" (Math|Transform|MakeTransform "0, 0, 0" "0, 0, 0" "1.000000,1.000000,1.000000") "Undefined" "MultiplyWithRoot" 0 (Variables|Default|GetPlayerCursor) 0))
      (Variables|Default|SetWhistleVolume _returnvalue_6))
    (:then_1
      (Utilities|IsValid _returnvalue
        (:Is%20Valid
          (Input|AddMappingContext _returnvalue "/Game/Input/IMC_ClutterCamera.IMC_ClutterCamera" 0 "(bIgnoreAllPressedKeysUntilRelease=True,bForceImmediately=False,bNotifyUserSettings=False)")
          (Input|AddMappingContext _returnvalue "/Game/Input/IMC_ClutterPlayer.IMC_ClutterPlayer" 0 "(bIgnoreAllPressedKeysUntilRelease=True,bForceImmediately=False,bNotifyUserSettings=False)")
          (Input|AddMappingContext _returnvalue "/Game/Input/IMC_ClutterCursor.IMC_ClutterCursor" 0 "(bIgnoreAllPressedKeysUntilRelease=True,bForceImmediately=False,bNotifyUserSettings=False)"))))
    (:then_2
      (Variables|/Game/Blueprints/BP_ClutterCamera.BP_ClutterCamera_C|SetMoveTarget (Variables|Default|GetPlayerCamera) (Variables|Default|GetPlayerCharacter)))))

(event EventTick
  (params (DeltaSeconds :type Float%20%28single-precision%29)))

(fn ConstructionScript)

(fn GetCharacter
  (return (Variables|Default|GetPlayerCharacter)))

(fn GetCamera
  (return (Variables|Default|GetPlayerCamera)))