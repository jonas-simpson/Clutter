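; BP_IgnoreMouse is a component that tags its owning actor "IgnoreMouse" and tracks whether the clutter camera faces it from an allowed side.
; BeginPlay normalizes VisibleDir, adds the tag and caches the clutter camera after a short delay.
; Each Tick, it sets Enabled when the dot product of the camera-to-owner direction and VisibleDir is positive, and clears it otherwise.
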(event EventBeginPlay
  (Variables|Default|SetVisibleDir (Math|Vector|Normalize (Variables|Default|GetVisibleDir)))
  (bind _output_get (Variables|Default|SetOwner (Components|GetOwner)))
  (Utilities|Array|Add (Variables|/Script/Engine.Actor|GetTags _output_get) "IgnoreMouse")
  (Utilities|FlowControl|Delay 0.2)
  (Variables|Default|SetCamera (Variables|/Game/Blueprints/BP_ClutterCamera.BP_ClutterCamera_C|GetCamera (CallFunction|GetClutterCamera))))

(event EventTick
  (params (DeltaSeconds :type Float%20%28single-precision%29))
  (Utilities|IsValid (Variables|Default|GetCamera)
    (:Is%20Valid
      (if (> (Math|Vector|DotProduct (Math|Vector|GetUnitDirection(Vector) (Transformation|GetWorldLocation (Variables|Default|GetCamera)) (Transformation|GetActorLocation (Variables|Default|GetOwner))) (Variables|Default|GetVisibleDir)) 0.0)
        (Variables|Default|SetEnabled true)
        (else
          (Variables|Default|SetEnabled false))))))